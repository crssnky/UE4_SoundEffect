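; Music visualizer actor that, toggled by right mouse, plays BGM and animates a ring of instanced-mesh bars from audio spectrum analysis.
; A looping timer samples frequency magnitudes to reposition and stretch each bar while rotating the ring.
; A delayed TimeSynth spawns colored Niagara bursts on quarter notes.
; Hardcoded timers, set on every press, switch the burst shape between triangle, rectangle and circle.
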(event `Key|RightMouseButton`
  (params (Key :type "Key Structure"))
  (bind _bgm (`self.BGM`))
  (bind _timesynth (`self.TimeSynth`))
  (:`Pressed`
    (`|ExecutionSequence`
      (:`then_0`
        (`KismetSystemLibrary.K2_SetTimer` self "changeToRectangle" 133.0)
        (`KismetSystemLibrary.K2_SetTimer` self "changeToTriangle" 215.75)
        (`KismetSystemLibrary.K2_SetTimer` self "changeToRectangle" 236.850006)
        (`KismetSystemLibrary.K2_SetTimer` self "changeToCircle" 239.600006))
      (:`then_1`
        (`/Engine/EditorBlueprintResources/StandardMacros.FlipFlop`
          (:`A`
            (`AudioMixerBlueprintLibrary.StartAnalyzingOutput` null "DefaultSize" "Linear" "Hamming")
            (`AudioComponent.Play` _bgm 0.0)
            (bind _returnvalue (`KismetSystemLibrary.K2_SetTimerDelegate` (delegate `UpdateMAgnitude`) 0.05 true))
            (set `self.TimerHandleUpdateMagnitude` _returnvalue)
            (`|ExecutionSequence`
              (:`then_0`
                (`TimeSynthComponent.SetBPM` _timesynth 132.0))
              (:`then_1`
                (`TimeSynthComponent.AddQuantizationEventDelegate` _timesynth "QuarterNote" (delegate `Burst`))
                (`KismetSystemLibrary.K2_SetTimerDelegate` (delegate `ActiveTimer`) 4.0)
                (add `AudioComponent.OnAudioFinished` (`self.BGM`) (delegate `AudioFinished`)))
              (:`then_2`
                (`SceneComponent.SetVisibility` (`self.Widget`) false true))))
          (:`B`
            (`AudioMixerBlueprintLibrary.StopAnalyzingOutput` null)
            (`AudioComponent.Stop` _bgm)
            (`KismetSystemLibrary.K2_ClearAndInvalidateTimerHandle` (`self.TimerHandleUpdateMagnitude`))
            (`ActorComponent.Deactivate` (`self.TimeSynth`))
            (`SceneComponent.SetVisibility` (`self.Widget`) true true)))))))

(event `ActiveTimer`
  (`ActorComponent.Activate` (`self.TimeSynth`) false))

(event `AudioFinished`
  (`ActorComponent.Deactivate` (`self.TimeSynth`)))

(event `Burst`
  (params (QuantizationType :type "ETimeSynthEventQuantization Enum" :default "None") (NumBars :type Integer) (Beat :type "Float (double-precision)"))
  (bind _returnvalue (`NiagaraFunctionLibrary.SpawnSystemAtLocation` (`self.Niagara`) (`self.K2_GetActorLocation`) (struct :`Yaw` 180.0)))
  (`NiagaraComponent.SetNiagaraVariableLinearColor` _returnvalue "User.ParticleColor" (`self.color`)))

(event `UpdateMAgnitude`
  (bind _magnitudes (`AudioMixerBlueprintLibrary.GetMagnitudeForFrequencies` (`self.Frequencies`) null))
  (for (_array_element _array_index) _magnitudes
    (bind _returnvalue (* _array_index 30.0))
    (bind _returnvalue_2 (`KismetMathLibrary.DegSin` _returnvalue))
    (bind _returnvalue_3 (* _array_element 0.25))
    (bind _returnvalue_4 (* _returnvalue_3 50.0))
    (bind _returnvalue_5 (`KismetMathLibrary.DegCos` _returnvalue))
    (`InstancedStaticMeshComponent.UpdateInstanceTransform` (`self.InstancedStaticMesh`) _array_index (`KismetMathLibrary.MakeTransform` (`KismetMathLibrary.MakeVector` 0.0 (+ (* _returnvalue_2 300.0) (* _returnvalue_4 _returnvalue_2)) (+ (* 300.0 _returnvalue_5) (* _returnvalue_5 _returnvalue_4))) (`KismetMathLibrary.MakeRotator` (* _array_index 30.0)) (`KismetMathLibrary.MakeVector` 1.0 1.0 _returnvalue_3)) false true true)
    (`SceneComponent.K2_AddLocalRotation` (`self.InstancedStaticMesh`) (struct :`Roll` 0.25) false false)))

(fn `changeToCircle`
  (set `self.Niagara` "/Game/Fx/RoolingTriangle/BurstCircle.BurstCircle"))

(fn `changeToRectangle`
  (set `self.Niagara` "/Game/Fx/RoolingTriangle/BurstRectangle.BurstRectangle"))

(fn `changeToTriangle`
  (set `self.Niagara` "/Game/Fx/RoolingTriangle/BurstTriangle.BurstTriangle"))

(fn `UserConstructionScript`
  (for _index (range 1 13)
    (`KismetArrayLibrary.Array_Add` (`self.Frequencies`) (* _index 100.0))
    (bind _returnvalue (* _index 30.0))
    (`InstancedStaticMeshComponent.AddInstance` (`self.InstancedStaticMesh`) (`KismetMathLibrary.MakeTransform` (`KismetMathLibrary.MakeVector` 0.0 (* (`KismetMathLibrary.DegSin` _returnvalue) 200.0) (* 200.0 (`KismetMathLibrary.DegCos` _returnvalue))) (`KismetMathLibrary.MakeRotator` (* _index 30.0)) (1.0 1.0 0.0)))
    (set `self.Niagara` "/Game/Fx/RoolingTriangle/BurstTriangle.BurstTriangle")))